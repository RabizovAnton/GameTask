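; BP_Shape is a falling shape in GeometryCatcher that the player collects by touching it.
; Each tick it moves down in world space at FallSpeed, scaled by delta time, with sweep enabled.
; On overlap with BP_Player it destroys itself, then tells GameManager to increment the collected tally for its Color and update that color's count.
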(event EventBeginPlay)

(event Collision|EventActorBeginOverlap
  (params (OtherActor :type Actor%20Object%20Reference))
  (Utilities|Casting|CastToBP_Player OtherActor)
  (Actor|DestroyActor)
  (Default|IncrementShapesCollected (Variables|Default|GetGameManager) (Variables|Default|GetColor))
  (Default|UpdateCount (Variables|Default|GetGameManager) (Variables|Default|GetColor)))

(event EventTick
  (params (DeltaSeconds :type Float%20%28single-precision%29))
  (Transformation|AddActorWorldOffset (Math|Vector|MakeVector 0.0 0.0 (* (* DeltaSeconds (Variables|Default|GetFallSpeed)) -1.0)) true))

(fn ConstructionScript)